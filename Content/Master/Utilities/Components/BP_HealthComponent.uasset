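; Actor component that tracks an owner's health, handling damage, healing clamped to max, death state, and a hit flash.
; On BeginPlay it resets health and creates a dynamic material instance from slot 0 of the owner's skeletal mesh.
; Damage briefly sets that material's emissive color and intensity, then clears them after a delay.
; Damage and healing both broadcast OnHealthChanged; damage also passes the impact point and prints the current health.
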(event `self.ReceiveBeginPlay`
  (`self.ResetHealth`)
  (bind _output_get (set `self.RefToOwner` (`self.GetOwner`)))
  (bind _returnvalue (`Actor.GetComponentByClass` _output_get "/Script/Engine.SkeletalMeshComponent"))
  (`/Engine/EditorBlueprintResources/StandardMacros.IsValid` _returnvalue
    (:`Is Valid`
      (bind _returnvalue_2 (`PrimitiveComponent.CreateDynamicMaterialInstance` _returnvalue 0 null "None"))
      (set `self.FlashMaterial` _returnvalue_2))))

(event `FlashActor`
  (params (ActorDead :type Boolean))
  (bind _flashmaterial (`self.FlashMaterial`))
  (bind _flashmaterial_2 (`self.FlashMaterial`))
  (`MaterialInstanceDynamic.SetVectorParameterValue` _flashmaterial "EmissiveColor" (`self.FlashColor`))
  (`MaterialInstanceDynamic.SetScalarParameterValue` _flashmaterial "EmissiveMultiplier" (`self.FlashIntensity`))
  (`KismetSystemLibrary.Delay` (`self.FlashDuration`))
  (`MaterialInstanceDynamic.SetVectorParameterValue` :`self` _flashmaterial_2 :`ParameterName` "EmissiveColor")
  (`MaterialInstanceDynamic.SetScalarParameterValue` _flashmaterial_2 "EmissiveMultiplier" 0.0))

(fn `Heal`
  (params (Amount :type "Float (double-precision)"))
  (bind _maxhealth (`self.MaxHealth`))
  (bind _returnvalue (+ (`self.CurrentHealth`) Amount))
  (set `self.CurrentHealth` (`KismetMathLibrary.SelectFloat` _maxhealth _returnvalue (> _returnvalue _maxhealth)))
  (`self.OnHealthChanged` (`self.MaxHealth`) (`self.CurrentHealth`) (`self.IsDead`)))

(fn `ResetHealth`
  (set `self.CurrentHealth` (`self.MaxHealth`))
  (set `self.IsDead` false))

(fn `TakeDamage`
  (params (Amout :type "Float (double-precision)") (ImpactPoint :type "Vector Structure"))
  (bind _returnvalue (- (`self.CurrentHealth`) Amout))
  (if (not (`self.IsDead`))
    (bind _output_get (set `self.CurrentHealth` (`KismetMathLibrary.SelectFloat` 0.0 _returnvalue (<= _returnvalue 0.0))))
    (`KismetSystemLibrary.PrintString` (`KismetStringLibrary.Conv_DoubleToString` _output_get))
    (bind _output_get_2 (set `self.IsDead` (<= _output_get 0.0)))
    (`self.FlashActor` _output_get_2)
    (`self.OnHealthChanged` (`self.MaxHealth`) (`self.CurrentHealth`) (`self.IsDead`) ImpactPoint)))