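; BP_Sign is a placeable world sign that shows a room name and an optional direction indicator.
; The construction script writes the room name text and toggles the visibility of the Direction component.
; It maps the Up, Down, Left or Right setting to a roll angle on that component.
; The event graph holds only disabled stub events, so the sign has no runtime logic.
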(fn `UserConstructionScript`
  (`TextRenderComponent.K2_SetText` (`self.RoomName`) (`self.RoomNameText`))
  (`SceneComponent.SetVisibility` (`self.Direction`) (`self.VisibilityDirection`) false)
  (switch `/Game/Blueprints/WorldActors/E_DirectionSign` (`self.DirectionSign`)
    (:`NewEnumerator0`
      (set `self.DirectionRotation` 90.0))
    (:`NewEnumerator1`
      (set `self.DirectionRotation` -90.0))
    (:`NewEnumerator2`
      (set `self.DirectionRotation` 180.0))
    (:`NewEnumerator3`
      (set `self.DirectionRotation` 0.0)))
  (`SceneComponent.K2_SetRelativeRotation` (`self.Direction`) (`KismetMathLibrary.MakeRotator` (`self.DirectionRotation`)) false false))