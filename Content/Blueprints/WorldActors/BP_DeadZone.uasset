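; BP_DeadZone is a world actor whose box trigger sends the player's BP_DialogueCharacter back to a respawn point on overlap.
; The respawn point is the player character's location recorded at BeginPlay.
; Overlap creates a WBP_Fade widget, starts its fade animation, moves the character immediately, then removes the widget after a delay matching the animation's end time.
; The construction script loops over a RespawnPoints count with an empty body.
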(event `self.ReceiveBeginPlay`
  (bind _asbp_dialogue_character (cast `/Game/Blueprints/Player/BP_DialogueCharacter` (`GameplayStatics.GetPlayerCharacter` 0)))
  (set `self.RespawnPoint` (`self.K2_GetActorLocation` _asbp_dialogue_character)))

(event `self.Box.OnComponentBeginOverlap`
  (params (OverlappedComponent :type "PrimitiveComponent Object Reference") (OtherActor :type "Actor Object Reference") (OtherComp :type "PrimitiveComponent Object Reference") (OtherBodyIndex :type Integer) (bFromSweep :type Boolean) (SweepResult :type "HitResult Structure (by ref)"))
  (bind _fadewidget (`self.FadeWidget`))
  (bind _fadeinout (`/Game/UI/Widgets/WBP_Fade.FadeInOut` _fadewidget))
  (bind _asbp_dialogue_character (cast `/Game/Blueprints/Player/BP_DialogueCharacter` OtherActor))
  (bind _returnvalue (`|CreateWidget` "/Game/UI/Widgets/WBP_Fade.WBP_Fade_C"))
  (bind _output_get (set `self.FadeWidget` _returnvalue))
  (`UserWidget.AddToViewport` _output_get -1)
  (`Image.SetColorAndOpacity` :`self` (`/Game/UI/Widgets/WBP_Fade.Image_0` _output_get))
  (`UserWidget.PlayAnimation` _fadewidget _fadeinout 0.0 1 "Forward" (`self.FadePlayRate`) false)
  (`self.K2_SetActorLocation` _asbp_dialogue_character (`self.RespawnPoint`) false false)
  (`KismetSystemLibrary.Delay` (`WidgetAnimation.GetEndTime` _fadeinout))
  (`Widget.RemoveFromParent` (`self.FadeWidget`)))

(fn `UserConstructionScript`
  (for _ (range (`self.RespawnPoints`))
    _))