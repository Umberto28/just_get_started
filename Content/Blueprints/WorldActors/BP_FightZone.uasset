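; Fight arena trigger volume that turns the dialogue character's movement into a side-view duel against BoldGuy.
; On entry it swaps music, plane-locks the player, blends to a camera tracking them along Y and enables fight input.
; The first visit plays story dialogue, later ones a countdown; a NoFight variant updates main-menu progress instead.
; Leaving restores player, camera and music and resets the fight; the visited flag uses the game instance.
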(event `self.ReceiveBeginPlay`
  (set `self.DefaultCameraPos` (`SceneComponent.K2_GetComponentLocation` (`self.SpringArm`)))
  (bind _asbp_player_controller (cast `/Game/Blueprints/Player/BP_PlayerController` (`GameplayStatics.GetPlayerController` 0)))
  (set `self.Controller` _asbp_player_controller)
  (bind _returnvalue (`GameplayStatics.GetActorOfClass` "/Game/Blueprints/Player/BP_DialogueCharacter.BP_DialogueCharacter_C"))
  (`/Engine/EditorBlueprintResources/StandardMacros.IsValid` _returnvalue
    (:`Is Valid`
      (set `self.RefToCharacter` _returnvalue)
      (`self.LoadData`)
      (if (not (`self.NoFight`))
        (bind _returnvalue_2 (`GameplayStatics.GetActorOfClass` "/Game/Blueprints/Characters/BoldGuy/BP_BoldGuy.BP_BoldGuy_C"))
        (`/Engine/EditorBlueprintResources/StandardMacros.IsValid` _returnvalue_2
          (:`Is Valid`
            (set `self.BoldGuy` _returnvalue_2)
            (bind _returnvalue_3 (`|CreateWidget` "/Game/UI/Widgets/WBP_FightUI.WBP_FightUI_C"))
            (bind _output_get (set `self.FightUI` _returnvalue_3))
            (`UserWidget.AddToViewport` _output_get 0)
            (`self.ResetFight`)))))))

(event `self.ReceiveTick`
  (params (DeltaSeconds :type "Float (single-precision)"))
  (bind (_defaultcamerapos_x _defaultcamerapos_y _defaultcamerapos_z) (`KismetMathLibrary.BreakVector` (`self.DefaultCameraPos`)))
  (bind (_returnvalue_x _returnvalue_y) (`KismetMathLibrary.BreakVector` (`self.K2_GetActorLocation` (`self.RefToCharacter`))))
  (`SceneComponent.K2_SetWorldLocation` (`self.SpringArm`) (`KismetMathLibrary.MakeVector` _defaultcamerapos_x _returnvalue_y _defaultcamerapos_z) false false))

(event `self.Box.OnComponentBeginOverlap`
  (params (OverlappedComponent :type "PrimitiveComponent Object Reference") (OtherActor :type "Actor Object Reference") (OtherComp :type "PrimitiveComponent Object Reference") (OtherBodyIndex :type Integer) (bFromSweep :type Boolean) (SweepResult :type "HitResult Structure (by ref)"))
  (bind _reftocharacter (`self.RefToCharacter`))
  (bind _boldguy (`self.BoldGuy`))
  (bind _charactermovement (`Character.CharacterMovement` _reftocharacter))
  ; Handle Collisions with Player
  (cast `/Game/Blueprints/Player/BP_DialogueCharacter` OtherActor)
  (bind _returnvalue (`GameplayStatics.GetActorOfClass` "/Game/UI/Blueprints/BP_SliderMusic.BP_SliderMusic_C"))
  (`/Game/UI/Blueprints/BP_SliderMusic.ChangeMusic` _returnvalue "/Game/Sounds/FightMusic.FightMusic")
  (`self.K2_SetActorLocation` _reftocharacter (`SceneComponent.K2_GetComponentLocation` (`self.PlayerPos`)) false false)
  (`MovementComponent.SetPlaneConstraintNormal` _charactermovement (1.0 0.0 0.0))
  (set `CharacterMovementComponent.JumpZVelocity` (`self.JumpForceOn`) _charactermovement)
  (set `CharacterMovementComponent.bOrientRotationToMovement` true _charactermovement)
  (`PlayerController.SetViewTargetWithBlend` (`self.Controller`) self (`self.BlendTime`) "VTBlend_Linear" 0.0 false)
  (`self.SetActorTickEnabled` true)
  (`/Game/Blueprints/Player/BP_PlayerController.FightInputOn` (`self.Controller`))
  (if (`self.NoFight`)
    (if (not (`self.Visited`))
      (bind _asbp_dialogue_game_mode (cast `/Game/Blueprints/Core/BP_DialogueGameMode` (`GameplayStatics.GetGameMode`)))
      (`/Game/Blueprints/Core/BP_DialogueGameMode.StartDialogueSequence` :`self` _asbp_dialogue_game_mode)
      (`self.UpdateStartButton`)
      (set `self.Visited` true :!label _label))
    (else
      (`/Engine/EditorBlueprintResources/StandardMacros.IsValid` _boldguy
        (:`Is Valid`
          (`/Game/Blueprints/Characters/BoldGuy/BP_BoldGuy.RunBT` _boldguy)
          (`Widget.SetVisibility` (`self.FightUI`) "Visible")
          (`CharacterMovementComponent.DisableMovement` (`Character.CharacterMovement` (`self.BoldGuy`)))
          (`CharacterMovementComponent.DisableMovement` (`Character.CharacterMovement` (`self.RefToCharacter`)))
          (if (not (`self.Visited`))
            (bind _asbp_dialogue_game_mode_2 (cast `/Game/Blueprints/Core/BP_DialogueGameMode` (`GameplayStatics.GetGameMode`)))
            (`/Game/Blueprints/Core/BP_DialogueGameMode.StartDialogueSequence` _asbp_dialogue_game_mode_2 (struct :`TagName` "StoryTags.BoldFight"))
            (set `/Game/Blueprints/Player/BP_PlayerController.IsInFight` true (`self.Controller`))
            (goto _label)
            (else
              (`self.StartFightAnim`))))))))

(event `self.Box.OnComponentEndOverlap`
  (params (OverlappedComponent :type "PrimitiveComponent Object Reference") (OtherActor :type "Actor Object Reference") (OtherComp :type "PrimitiveComponent Object Reference") (OtherBodyIndex :type Integer))
  ; Handle Collisions with Player
  (bind _asbp_dialogue_character (cast `/Game/Blueprints/Player/BP_DialogueCharacter` OtherActor))
  (`self.PlayerOutOfBox` _asbp_dialogue_character)
  (bind _returnvalue (`GameplayStatics.GetActorOfClass` "/Game/UI/Blueprints/BP_SliderMusic.BP_SliderMusic_C"))
  (`/Game/UI/Blueprints/BP_SliderMusic.ChangeMusic` _returnvalue "/Game/Sounds/01_Zero-It-Out_Main_Theme.01_Zero-It-Out_Main_Theme"))

(event `/Game/Blueprints/Interfaces/BPI_SaveInterface.LoadData`
  ; Saving
  (bind _asgi_started (cast `/Game/Blueprints/Core/GI_Started` (`GameplayStatics.GetGameInstance`)))
  (set `self.Visited` (`/Game/Blueprints/Core/GI_Started.FightZoneVisited` _asgi_started)))

(event `StartFightAnim`
  (bind _fightui (`self.FightUI`))
  (bind _countdown (`/Game/UI/Widgets/WBP_FightUI.CountDown` _fightui))
  (`UserWidget.PlayAnimation` _fightui _countdown 0.0 1 "Forward" 1.0 false)
  (`KismetSystemLibrary.Delay` (`WidgetAnimation.GetEndTime` _countdown))
  (`CharacterMovementComponent.SetMovementMode` (`Character.CharacterMovement` (`self.BoldGuy`)) "MOVE_Walking" 0)
  (`CharacterMovementComponent.SetMovementMode` (`Character.CharacterMovement` (`self.RefToCharacter`)) "MOVE_Walking" 0))

(event `/Game/Blueprints/Interfaces/BPI_SaveInterface.SaveData`
  ; Saving
  (bind _asgi_started (cast `/Game/Blueprints/Core/GI_Started` (`GameplayStatics.GetGameInstance`)))
  (set `/Game/Blueprints/Core/GI_Started.FightZoneVisited` (`self.Visited`) _asgi_started))

(fn `PlayerOutOfBox`
  (params (NewViewTarget :type "Actor Object Reference"))
  (bind _charactermovement (`Character.CharacterMovement` (`self.RefToCharacter`)))
  (`MovementComponent.SetPlaneConstraintNormal` _charactermovement (0.0 0.0 0.0))
  (set `CharacterMovementComponent.JumpZVelocity` (`self.JumpoForceOff`) _charactermovement)
  (set `CharacterMovementComponent.bOrientRotationToMovement` false _charactermovement)
  (`PlayerController.SetViewTargetWithBlend` (`self.Controller`) NewViewTarget (`self.BlendTime`) "VTBlend_Linear" 0.0 false)
  (`/Game/Blueprints/Player/BP_PlayerController.FightInputOff` (`self.Controller`))
  (`self.ResetFight`))

(fn `ResetFight`
  (`/Game/Master/Utilities/Components/BP_HealthComponent.ResetHealth` (`/Game/Blueprints/Characters/BoldGuy/BP_BoldGuy.BP_HealthComponent` (`self.BoldGuy`)))
  (`/Game/Master/Utilities/Components/BP_HealthComponent.ResetHealth` (`/Game/Blueprints/Player/BP_DialogueCharacter.BP_HealthComponent` (`self.RefToCharacter`)))
  (`self.UpdateHealthBar` 1.0 true)
  (`self.UpdateHealthBar` 1.0)
  (`self.K2_SetActorTransform` (`self.BoldGuy`) (`KismetMathLibrary.MakeTransform` (`SceneComponent.K2_GetComponentLocation` (`self.EnemyPos`)) (struct :`Yaw` 90.0)) false false)
  (`Widget.SetVisibility` (`self.FightUI`) "Hidden"))

(fn `UpdateHealthBar`
  (params (Health :type "Float (double-precision)") (IsPlayer :type Boolean))
  (bind _fightui (`self.FightUI`))
  (if IsPlayer
    (`ProgressBar.SetPercent` (`/Game/UI/Widgets/WBP_FightUI.PlayerProgressBar` _fightui) Health)
    (else
      (`ProgressBar.SetPercent` (`/Game/UI/Widgets/WBP_FightUI.EnemyProgressBar` _fightui) Health))))

(fn `UpdateStartButton`
  (bind _returnvalue (`GameplayStatics.GetActorOfClass` "/Game/UI/Blueprints/BP_ToggleShyMode.BP_ToggleShyMode_C"))
  (`/Engine/EditorBlueprintResources/StandardMacros.IsValid` _returnvalue
    (:`Is Valid`
      (set `/Game/UI/Blueprints/BP_ToggleShyMode.BoldDefeated` true _returnvalue)
      (bind _returnvalue_2 (`GameplayStatics.GetActorOfClass` "/Game/UI/Blueprints/BP_MainMenu.BP_MainMenu_C"))
      (`/Engine/EditorBlueprintResources/StandardMacros.IsValid` _returnvalue_2
        (:`Is Valid`
          (bind _aswbp_main_menu_composition (cast `/Game/UI/Widgets/WBP_MainMenuComposition` (`WidgetComponent.GetWidget` (`/Game/UI/Blueprints/BP_MainMenu.MenuWidget` _returnvalue_2))))
          (if (`|EnumEquality` (`/Game/UI/Widgets/WBP_MainMenuComposition.StartButtonMode` _aswbp_main_menu_composition) "NewEnumerator1")
            (set `/Game/UI/Widgets/WBP_MainMenuComposition.StartButtonMode` "NewEnumerator2" _aswbp_main_menu_composition)))))))

(fn `UserConstructionScript`
  (bind _springarm (`self.SpringArm`))
  (`SceneComponent.K2_SetRelativeLocation` _springarm (`KismetMathLibrary.MakeVector` 0.0 0.0 (`self.CameraZ`)) false false)
  (set `SpringArmComponent.TargetArmLength` (`self.CameraX`) _springarm))