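; Puppet theater puzzle actor that switches the view to its own camera and fades its floor material while the dialogue character stands inside TheaterBox.
; On tick, the character's movement drives the hidden-until-entry puppet opposite to the character's forward vector.
; The puppet reaching SecretBox opens the secret door and marks the puzzle solved.
; Leaving resets the puppet, or removes puppet and door once solved; solved state persists through GI_Started.
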(event `self.ReceiveBeginPlay`
  (bind _returnvalue (`GameplayStatics.GetActorOfClass` "/Game/Blueprints/Characters/Puppet/BP_Puppet.BP_Puppet_C"))
  (`/Engine/EditorBlueprintResources/StandardMacros.IsValid` _returnvalue
    (:`Is Valid`
      (set `self.RefToPuppet` _returnvalue)
      (`self.ResetPuppet`))))

(event `/Game/Blueprints/Interfaces/BPI_SaveInterface.SaveData`
  ; Savings
  (bind _asgi_started (cast `/Game/Blueprints/Core/GI_Started` (`GameplayStatics.GetGameInstance`)))
  (set `/Game/Blueprints/Core/GI_Started.PuppetSolved` (`self.Solved`) _asgi_started))

(event `self.ReceiveTick`
  (params (DeltaSeconds :type "Float (single-precision)"))
  (bind _reftocharacter (`self.RefToCharacter`))
  (if (> (`KismetMathLibrary.VSizeXY` (`MovementComponent.Velocity` (`Character.CharacterMovement` _reftocharacter))) 1.0)
    (`Pawn.AddMovementInput` (`self.RefToPuppet`) (* (`self.GetActorForwardVector` _reftocharacter) -1.0) (`self.MovementScale`) false)))

(event `MaterialSet`
  ; MaterialFade
  (if (and (`self.Entering?`) (not (`self.Solved`)))
    (bind (_direction _state) (`Timeline|FadeinFadeOut` :!label _label)
      (:`Update`
        (`MaterialInstanceDynamic.SetScalarParameterValue` (`self.RefToRealFloorMaterial`) "State" _state)))
    (else
      (goto _label :!via `Reverse`))))

(event `self.TheaterBox.OnComponentBeginOverlap`
  (params (OverlappedComponent :type "PrimitiveComponent Object Reference") (OtherActor :type "Actor Object Reference") (OtherComp :type "PrimitiveComponent Object Reference") (OtherBodyIndex :type Integer) (bFromSweep :type Boolean) (SweepResult :type "HitResult Structure (by ref)"))
  (bind _reftopuppet (`self.RefToPuppet`))
  ; Box Overlap Interactions
  (bind _asbp_dialogue_character (cast `/Game/Blueprints/Player/BP_DialogueCharacter` OtherActor))
  (set `self.RefToCharacter` _asbp_dialogue_character)
  (`PlayerController.SetViewTargetWithBlend` (`GameplayStatics.GetPlayerController` 0) self (`self.BlendTime`) "VTBlend_Linear" 0.0 false)
  (`/Engine/EditorBlueprintResources/StandardMacros.IsValid` _reftopuppet
    (:`Is Valid`
      (`self.SetActorHiddenInGame` _reftopuppet false)
      (`self.SetActorTickEnabled` true)
      (set `self.Entering?` true)
      (`self.MaterialSet` :!label _label_2))))

(event `self.TheaterBox.OnComponentEndOverlap`
  (params (OverlappedComponent :type "PrimitiveComponent Object Reference") (OtherActor :type "Actor Object Reference") (OtherComp :type "PrimitiveComponent Object Reference") (OtherBodyIndex :type Integer))
  ; Box Overlap Interactions
  (bind _asbp_dialogue_character (cast `/Game/Blueprints/Player/BP_DialogueCharacter` OtherActor))
  (`PlayerController.SetViewTargetWithBlend` (`GameplayStatics.GetPlayerController` 0) _asbp_dialogue_character (`self.BlendTime`) "VTBlend_Linear" 0.0 false)
  (`self.SetActorTickEnabled` false)
  (set `self.Entering?` false)
  (if (`self.Solved`)
    (`self.SelfDestruction`)
    (goto _label_2)
    (else
      (`self.ResetPuppet`)
      (goto _label_2))))

(event `self.SecretBox.OnComponentBeginOverlap`
  (params (OverlappedComponent :type "PrimitiveComponent Object Reference") (OtherActor :type "Actor Object Reference") (OtherComp :type "PrimitiveComponent Object Reference") (OtherBodyIndex :type Integer) (bFromSweep :type Boolean) (SweepResult :type "HitResult Structure (by ref)"))
  (bind _secretdoor (`self.SecretDoor`))
  ; Secret Door
  (if (== OtherActor (`self.RefToPuppet`))
    (`/Engine/EditorBlueprintResources/StandardMacros.IsValid` _secretdoor
      (:`Is Valid`
        (`/Game/Blueprints/WorldActors/BP_SecretDoor.OpenDoor` _secretdoor)
        (set `self.Solved` true)
        (`ActorComponent.K2_DestroyComponent` (`self.StaticMesh`)))
      (:`Is Not Valid`
        (`KismetSystemLibrary.PrintString` "No Secret Door")))))

(fn `LoadDataSave`
  (params (IsSolved :type Boolean))
  (bind _output_get (set `self.Solved` IsSolved))
  (if _output_get
    (`self.SelfDestruction`)))

(fn `ResetPuppet`
  (bind _reftopuppet (`self.RefToPuppet`))
  (bind (_returnvalue_location _returnvalue_rotation) (`KismetMathLibrary.BreakTransform` (`SceneComponent.K2_GetComponentToWorld` (`self.StartingPos`))))
  (`/Engine/EditorBlueprintResources/StandardMacros.IsValid` _reftopuppet
    (:`Is Valid`
      (`self.K2_SetActorTransform` _reftopuppet (`KismetMathLibrary.MakeTransform` _returnvalue_location _returnvalue_rotation) false false)
      (`self.SetActorHiddenInGame` (`self.RefToPuppet`) true))))

(fn `SelfDestruction`
  (bind _reftopuppet (`self.RefToPuppet`))
  (bind _secretdoor (`self.SecretDoor`))
  (`/Engine/EditorBlueprintResources/StandardMacros.IsValid` _reftopuppet
    (:`Is Valid`
      (`self.K2_DestroyActor` _reftopuppet)
      (`PrimitiveComponent.SetCollisionEnabled` (`self.TheaterBox`) "NoCollision")
      (`PrimitiveComponent.SetCollisionEnabled` (`self.SecretBox`) "NoCollision")
      (`/Engine/EditorBlueprintResources/StandardMacros.IsValid` _secretdoor
        (:`Is Valid`
          (`self.K2_DestroyActor` _secretdoor))))))

(fn `UserConstructionScript`
  (bind _bp_puppettheaterlabyrint (`self.BP_PuppetTheaterLabyrint`))
  (bind _startingpos (`self.StartingPos`))
  (bind _secretbox (`self.SecretBox`))
  (bind (_relativelocation_x _relativelocation_y) (`KismetMathLibrary.BreakVector` (`SceneComponent.RelativeLocation` _secretbox)))
  (bind (_relativelocation_x_2 _relativelocation_y_2) (`KismetMathLibrary.BreakVector` (`SceneComponent.RelativeLocation` _startingpos)))
  (bind (_relativelocation_x_3 _relativelocation_y_3) (`KismetMathLibrary.BreakVector` (`SceneComponent.RelativeLocation` _bp_puppettheaterlabyrint)))
  (`SceneComponent.K2_SetRelativeLocation` _startingpos (`KismetMathLibrary.MakeVector` _relativelocation_x_2 _relativelocation_y_2 (`self.PuppetZ`)) false false)
  (`SceneComponent.K2_SetRelativeLocation` _secretbox (`KismetMathLibrary.MakeVector` _relativelocation_x _relativelocation_y (`self.PuppetZ`)) false false)
  (`SceneComponent.K2_SetRelativeLocation` (`self.Camera`) (`KismetMathLibrary.MakeVector` (`self.CameraHeight`)) false false)
  (`SceneComponent.K2_SetRelativeLocation` _bp_puppettheaterlabyrint (`KismetMathLibrary.MakeVector` _relativelocation_x_3 _relativelocation_y_3 (- (`self.PuppetZ`) 18.0)) false false)
  (bind _returnvalue (`PrimitiveComponent.CreateDynamicMaterialInstance` (`self.RealFloor`) 0 "/Game/Materials/MaterialIstances/MI_Sound_ControlRoom.MI_Sound_ControlRoom" "None"))
  (bind _output_get (set `self.RefToRealFloorMaterial` _returnvalue))
  (`PrimitiveComponent.SetMaterial` (`self.RealFloor`) 0 _output_get))