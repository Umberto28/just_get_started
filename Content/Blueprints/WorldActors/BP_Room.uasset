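; BP_Room is a room trigger volume that shows its contents while a dialogue character is inside and starts a dialogue sequence on first entry.
; The actors in ActorsToHandle start hidden, become visible when a BP_DialogueCharacter overlaps RoomCollision, and are hidden again when the overlap ends.
; The first overlap passes SequenceTag to BP_DialogueGameMode's StartDialogueSequence and sets Visited so it does not replay.
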(event `self.ReceiveBeginPlay`
  (bind _asbp_dialogue_game_mode (cast `/Game/Blueprints/Core/BP_DialogueGameMode` (`GameplayStatics.GetGameMode`)))
  (set `self.GameMode` _asbp_dialogue_game_mode)
  (if (`KismetArrayLibrary.Array_IsNotEmpty` (`self.ActorsToHandle`))
    (`self.DisableActors`)))

(event `self.RoomCollision.OnComponentBeginOverlap`
  (params (OverlappedComponent :type "PrimitiveComponent Object Reference") (OtherActor :type "Actor Object Reference") (OtherComp :type "PrimitiveComponent Object Reference") (OtherBodyIndex :type Integer) (bFromSweep :type Boolean) (SweepResult :type "HitResult Structure (by ref)"))
  (cast `/Game/Blueprints/Player/BP_DialogueCharacter` OtherActor)
  (`self.EnableActors`)
  (if (not (`self.Visited`))
    (`/Game/Blueprints/Core/BP_DialogueGameMode.StartDialogueSequence` (`self.GameMode`) (`self.SequenceTag`))
    (set `self.Visited` true)))

(event `self.RoomCollision.OnComponentEndOverlap`
  (params (OverlappedComponent :type "PrimitiveComponent Object Reference") (OtherActor :type "Actor Object Reference") (OtherComp :type "PrimitiveComponent Object Reference") (OtherBodyIndex :type Integer))
  (cast `/Game/Blueprints/Player/BP_DialogueCharacter` OtherActor)
  (`self.DisableActors`))

(fn `DisableActors`
  (for _array_element (`self.ActorsToHandle`)
    (`/Engine/EditorBlueprintResources/StandardMacros.IsValid` _array_element
      (:`Is Valid`
        (`self.SetActorHiddenInGame` _array_element true)))))

(fn `EnableActors`
  (for _array_element (`self.ActorsToHandle`)
    (`/Engine/EditorBlueprintResources/StandardMacros.IsValid` _array_element
      (:`Is Valid`
        (`self.SetActorHiddenInGame` _array_element false)))))

(fn `UserConstructionScript`)