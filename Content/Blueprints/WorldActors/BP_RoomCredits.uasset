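; BP_RoomCredits is the credits room actor, which tracks whether that room has been visited through the game instance.
; On BeginPlay it runs the parent logic, then LoadData copies the Credits entry of RoomsVisited from GI_Started into Visited.
; SaveData writes back by assigning a newly made SRoomList built from Visited alone, replacing the whole struct rather than updating one field.
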(event `self.ReceiveBeginPlay`
  (`parent.ReceiveBeginPlay`)
  (`/Game/Blueprints/Interfaces/BPI_SaveInterface.LoadData`))

(event `self.LoadData`
  (bind _asgi_started (cast `/Game/Blueprints/Core/GI_Started` (`GameplayStatics.GetGameInstance`)))
  (set `self.Visited` (`.Credits_10_B4A8C19240F5B32FCC269AA3EAE2253E` (break `/Game/Blueprints/S_RoomList` (`/Game/Blueprints/Core/GI_Started.RoomsVisited` _asgi_started)))))

(event `self.SaveData`
  (bind _asgi_started (cast `/Game/Blueprints/Core/GI_Started` (`GameplayStatics.GetGameInstance`)))
  (set `/Game/Blueprints/Core/GI_Started.RoomsVisited` (make `/Game/Blueprints/S_RoomList` :`Credits` (`self.Visited`)) _asgi_started))

(fn `UserConstructionScript`
  (`parent.UserConstructionScript`))