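; A trigger platform actor that changes the level's post-process settings when a BP_DialogueCharacter steps into its box.
; On BeginPlay it finds a PostProcessVolume and fills a blendable array with its assigned post-process material at full weight.
; Overlap replaces the volume's whole settings struct with the result of CreateSettings, and nothing restores it on exit.
; The construction script shows the material's text on a TextRender label.
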(event `self.ReceiveBeginPlay`
  (bind _returnvalue (`GameplayStatics.GetActorOfClass` "/Script/Engine.PostProcessVolume"))
  (set `self.PostProcess` _returnvalue)
  (`KismetArrayLibrary.Array_Clear` (`self.BlendableArray`))
  (bind _output_get (set `self.NewBlendable` (make `WeightedBlendable` 1.0 (`self.PostProcessMaterial`))))
  (`KismetArrayLibrary.Array_AddUnique` (`self.BlendableArray`) _output_get))

(event `self.Box.OnComponentBeginOverlap`
  (params (OverlappedComponent :type "PrimitiveComponent Object Reference") (OtherActor :type "Actor Object Reference") (OtherComp :type "PrimitiveComponent Object Reference") (OtherBodyIndex :type Integer) (bFromSweep :type Boolean) (SweepResult :type "HitResult Structure (by ref)"))
  (cast `/Game/Blueprints/Player/BP_DialogueCharacter` OtherActor)
  (set `PostProcessVolume.Settings` (make `PostProcessSettings` :`WeightedBlendables` (make `WeightedBlendables` (`self.BlendableArray`))) (`self.PostProcess`)))

(fn `UserConstructionScript`
  (`TextRenderComponent.K2_SetText` (`self.TextRender`) (`self.MaterialText`)))