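; Main menu camera actor that lets the player interact with the widget held by BP_MainMenu.
; Its construction script positions it relative to that actor, using the actor's forward vector, MenuDistance and ZOffset.
; BeginPlay caches the menu widget and BP_DialogueGameMode; SetControllerInput enables input and focuses the widget in Game and UI mode.
; StartWidget and EndWidget simulate left-mouse press and release through a WidgetInteraction component.
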(event `self.ReceiveBeginPlay`
  (bind _returnvalue (`GameplayStatics.GetActorOfClass` "/Game/UI/Blueprints/BP_MainMenu.BP_MainMenu_C"))
  (set `self.RefToWidget` (`/Game/UI/Blueprints/BP_MainMenu.MenuWidget` _returnvalue))
  (bind _asbp_dialogue_game_mode (cast `/Game/Blueprints/Core/BP_DialogueGameMode` (`GameplayStatics.GetGameMode`)))
  (set `self.RefToGameMode` _asbp_dialogue_game_mode))

(event `StartWidget`
  (`WidgetInteractionComponent.PressPointerKey` (`self.WidgetInteraction`) "LeftMouseButton"))

(event `EndWidget`
  (`WidgetInteractionComponent.ReleasePointerKey` (`self.WidgetInteraction`) "LeftMouseButton"))

(fn `SetControllerInput`
  (bind _returnvalue (`GameplayStatics.GetPlayerController` 0))
  (`self.EnableInput` _returnvalue)
  (`WidgetBlueprintLibrary.SetInputMode_GameAndUIEx` _returnvalue (`WidgetComponent.GetWidget` (`self.RefToWidget`)) "DoNotLock" false))

(fn `UserConstructionScript`
  (bind (_returnvalue_x _returnvalue_y) (`KismetMathLibrary.BreakVector` (`self.K2_GetActorLocation`)))
  (bind _returnvalue (`GameplayStatics.GetActorOfClass` "/Game/UI/Blueprints/BP_MainMenu.BP_MainMenu_C"))
  (`/Engine/EditorBlueprintResources/StandardMacros.IsValid` _returnvalue
    (:`Is Valid`
      (bind _returnvalue_2 (`self.K2_GetActorLocation` _returnvalue))
      (`self.K2_SetActorLocation` _returnvalue_2)
      (bind _returnvalue_3 (`self.GetActorForwardVector` _returnvalue))
      (bind (_returnvalue_x_2 _returnvalue_y_2) (`KismetMathLibrary.BreakVector` (+ (* _returnvalue_3 _returnvalue_2) (* _returnvalue_3 (`self.MenuDistance`)))))
      (`self.K2_SetActorLocation` (`KismetMathLibrary.MakeVector` (+ _returnvalue_x _returnvalue_x_2) (+ _returnvalue_y _returnvalue_y_2) (+ (.z _returnvalue_2) (`self.ZOffset`)))))))