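; Game mode that runs tagged dialogue sequences through an on-screen dialogue box.
; On BeginPlay it creates hidden dialogue and interaction message widgets and caches the main menu camera.
; StartDialogueSequence scans DT_DialoguesTable for the matching tag, loads its lines and quit flags, and disables the camera's widget interaction.
; TextInteract skips typing or advances lines, then reverses the pop-up and restores widget interaction after the last line.
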(event `self.ReceiveBeginPlay`
  (bind _returnvalue (`GameplayStatics.GetPlayerController` 0))
  (bind _returnvalue_2 (`|CreateWidget` "/Game/UI/Widgets/WBP_DialogueBox.WBP_DialogueBox_C" _returnvalue))
  (bind _output_get (set `self.DialogueBox` _returnvalue_2))
  (`UserWidget.AddToViewport` _output_get 1)
  (`Widget.SetVisibility` _output_get "Hidden")
  (bind _returnvalue_3 (`|CreateWidget` "/Game/UI/Widgets/WBP_InteractionMessage.WBP_InteractionMessage_C" _returnvalue))
  (bind _output_get_2 (set `self.InteractionMessage` _returnvalue_3))
  (`UserWidget.AddToViewport` _output_get_2 0)
  (`Widget.SetVisibility` _output_get_2 "Hidden")
  (bind _returnvalue_4 (`GameplayStatics.GetActorOfClass` "/Game/Blueprints/Player/BP_MainMenuCamera.BP_MainMenuCamera_C"))
  (`/Engine/EditorBlueprintResources/StandardMacros.IsValid` _returnvalue_4
    (:`Is Valid`
      (set `self.RefToMainCamera` _returnvalue_4))))

(event `StartDialogueSequence`
  (params (SequenceTag :type "GameplayTag Structure"))
  (bind _dialoguebox (`self.DialogueBox`))
  (bind _reftomaincamera (`self.RefToMainCamera`)
    (:`then`
      (`ActorComponent.Deactivate` (`/Game/Blueprints/Player/BP_MainMenuCamera.WidgetInteraction` _reftomaincamera)))
    (:`else`
      _))
  (bind _outrownames (`DataTableFunctionLibrary.GetDataTableRowNames` "/Game/DialogueAssets/DT_DialoguesTable.DT_DialoguesTable"))
  (bind _output_get (set `self.RowNames` _outrownames))
  (for _array_element _output_get
    (bind _returnvalue (`|GetDataTableRow` "/Game/DialogueAssets/DT_DialoguesTable.DT_DialoguesTable" _array_element)
      (:`then`
        (bind (_sequencetag _dialoguelines _faceexpression _isquitgame _quitanyway) (break `/Game/DialogueAssets/S_Dialogue` _returnvalue))
        (if (== _sequencetag SequenceTag)
          (set `self.Is Quit Game` _isquitgame)
          (set `self.Quit Anyway` _quitanyway)
          (set `self.Dialogue Lines` _dialoguelines)))))
  (if (`KismetArrayLibrary.Array_IsEmpty` (`self.Dialogue Lines`))
    (`KismetSystemLibrary.PrintString` "ERROR: LINES ARRAY NOT FOUND OR EMPTY" true true (struct :`R` 1.0 :`G` 2.4e-05 :`B` 0.004985 :`A` 1.0) 5.0)
    (else
      (`Widget.SetVisibility` _dialoguebox "Visible")
      (set `self.CurrentDialogueLineIndex` 0)
      (`/Game/UI/Widgets/WBP_DialogueBox.PlayPopUpAnimationAndSetText` _dialoguebox false (`KismetTextLibrary.Conv_StringToText` (`|GetArrayItem` (`self.Dialogue Lines`))) (`self.Is Quit Game`) (`self.Quit Anyway`)))))

(event `TextInteract`
  (bind _dialoguebox (`self.DialogueBox`))
  (bind _dialoguebox_2 (`self.DialogueBox`))
  (if (`Widget.IsVisible` _dialoguebox)
    (switch `/Game/DialogueAssets/E_DialogueBoxState` (`/Game/UI/Widgets/WBP_DialogueBox.CurrentState` _dialoguebox)
      (:`NewEnumerator0`
        (bind _result (`/Engine/EditorBlueprintResources/StandardMacros.IncrementInt` (`self.CurrentDialogueLineIndex`))
          (:`  `
            (if (< _result (`KismetArrayLibrary.Array_Length` (`self.Dialogue Lines`)))
              (`/Game/UI/Widgets/WBP_DialogueBox.SetDialogueText` _dialoguebox (`KismetTextLibrary.Conv_StringToText` (`|GetArrayItem` (`self.Dialogue Lines`) (`self.CurrentDialogueLineIndex`))))
              (else
                (`/Game/UI/Widgets/WBP_DialogueBox.StopTimer` _dialoguebox_2)
                (`/Game/UI/Widgets/WBP_DialogueBox.PlayPopUpAnimationAndSetText` _dialoguebox_2 true "" false false)
                (bind _reftomaincamera (`self.RefToMainCamera`)
                  (:`then`
                    (`ActorComponent.Activate` (`/Game/Blueprints/Player/BP_MainMenuCamera.WidgetInteraction` _reftomaincamera) false))
                  (:`else`)))))))
      (:`NewEnumerator1`
        (`/Game/UI/Widgets/WBP_DialogueBox.SkipTimer` _dialoguebox)))))

(fn `UserConstructionScript`)