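; BP_BoldGuy is an AI melee opponent that runs the BT_BoldGuy behavior tree and reports to the level's BP_FightZone.
; Attacks pick one of two animation indices behind an IsAttacking guard, while StartAttack and EndCollision toggle the hit box's trace-channel response.
; Box overlaps damage any actor with a BP_HealthComponent.
; Health changes update the zone's enemy bar; death disables movement, and Defeated updates the start button before destroying the actor.
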(event `RunBT`
  (bind _asbp_aicontroller (cast `/Game/Blueprints/Characters/BP_AIController` (`self.GetController`)))
  (`AIController.RunBehaviorTree` _asbp_aicontroller "/Game/Blueprints/Characters/BoldGuy/BT_BoldGuy.BT_BoldGuy")
  (bind _returnvalue (`GameplayStatics.GetActorOfClass` "/Game/Blueprints/WorldActors/BP_FightZone.BP_FightZone_C"))
  (`/Engine/EditorBlueprintResources/StandardMacros.IsValid` _returnvalue
    (:`Is Valid`
      (set `self.FightZone` _returnvalue)
      (add `/Game/Master/Utilities/Components/BP_HealthComponent.OnHealthChanged` (`self.BP_HealthComponent`) (delegate `HealthChanged`)))))

(event `HealthChanged`
  (params (MaxHealth :type "Float (double-precision)") (CurrentHealth :type "Float (double-precision)") (IsDead :type Boolean) (ImpactPoint :type "Vector Structure"))
  (`/Game/Blueprints/WorldActors/BP_FightZone.UpdateHealthBar` (`self.FightZone`) (/ CurrentHealth MaxHealth) false)
  (if IsDead
    (`CharacterMovementComponent.DisableMovement` (`self.CharacterMovement`))))

(event `StartAttack`
  (`PrimitiveComponent.SetCollisionResponseToChannel` (`self.Box`) "ECC_GameTraceChannel1" "ECR_Overlap"))

(event `EndCollision`
  (`PrimitiveComponent.SetCollisionResponseToChannel` (`self.Box`) "ECC_GameTraceChannel1" "ECR_Ignore"))

(event `AttackAnimation`
  (if (not (`self.IsAttacking`))
    (set `self.RandomIdxAnim` (`KismetMathLibrary.RandomIntegerInRange` 0 1))
    (set `self.IsAttacking` true)
    (`KismetSystemLibrary.Delay` 1.8)
    (set `self.IsAttacking` false)))

(event `self.Box.OnComponentBeginOverlap`
  (params (OverlappedComponent :type "PrimitiveComponent Object Reference") (OtherActor :type "Actor Object Reference") (OtherComp :type "PrimitiveComponent Object Reference") (OtherBodyIndex :type Integer) (bFromSweep :type Boolean) (SweepResult :type "HitResult Structure (by ref)"))
  (bind _returnvalue (`self.GetComponentByClass` OtherActor "/Game/Master/Utilities/Components/BP_HealthComponent.BP_HealthComponent_C"))
  (`/Engine/EditorBlueprintResources/StandardMacros.IsValid` _returnvalue
    (:`Is Valid`
      (`/Game/Master/Utilities/Components/BP_HealthComponent.TakeDamage` _returnvalue (`self.Damage`) (0.0 0.0 0.0)))))

(fn `AttackPlayer`
  (if (not (`self.IsAttacking`))
    (set `self.RandomIdxAnim` (`KismetMathLibrary.RandomIntegerInRange` 0 1))
    (set `self.IsAttacking` true)))

(fn `Defeated`
  (`/Game/Blueprints/WorldActors/BP_FightZone.UpdateStartButton` (`self.FightZone`))
  (`self.K2_DestroyActor`))

(fn `UserConstructionScript`)